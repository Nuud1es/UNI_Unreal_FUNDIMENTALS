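; StandOnPlatform is a trigger actor that moves a cube when another actor overlaps it.
; On BeginPlay it spawns a MoveableCube at its Cylinder component's world location and keeps a reference to it.
; Each begin-overlap prints a debug greeting and shifts that cube a fixed step along world Y, without sweep.
; An offset vector built from the cylinder's location is left unused.
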(event Collision|EventActorBeginOverlap
  (params (OtherActor :type Actor%20Object%20Reference))
  ;[1 1 1] On overlap move object
  (Development|PrintString "Hello")
  (Transformation|AddActorWorldOffset (Variables|Default|GetCubeRef) "0.000000,20.000000,0.000000"))

(event EventBeginPlay
  ;[1 1 1] Spawns the Moveable Cube to get reference
  (bind _returnvalue (Game|SpawnActorfromClass "/Game/Blueprints/SomethingThatMoves/MoveableCube.MoveableCube_C" (Math|Transform|MakeTransform (Transformation|GetWorldLocation (Variables|Default|GetCylinder)) "0, 0, 0" "1.000000,1.000000,1.000000") "Undefined" 0 0))
  (Variables|Default|SetCubeRef _returnvalue))

(fn ConstructionScript)