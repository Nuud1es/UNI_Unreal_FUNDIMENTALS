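; SpawnPad is a pad actor that spawns a Light actor just above itself when play begins.
; On BeginPlay it offsets the SpawnPad component's world location upward, spawns the Light there and stores it in LightReF.
; It then enables input from the first player controller, though its graphs contain no input events and make no further use of the stored light.
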(event EventBeginPlay
  (bind _spawnpad (Variables|Default|GetSpawnPad))
  (bind _returnvalue (Transformation|GetWorldLocation _spawnpad))
  (bind (_x _y _z) (Class|KismetMathLibrary|BreakVector3f _returnvalue))
  (Utilities|FlowControl|Sequence
    (:then_0
      (bind _returnvalue_2 (Game|SpawnActorfromClass "/Game/Blueprints/LightThatChangesColour/Light.Light_C" (Math|Conversions|ToTransform(Vector) (Math|Vector|MakeVector _x _y (+ _z 3e+01))) "Undefined" 0 0))
      (Variables|Default|SetLight%20ReF _returnvalue_2))
    (:then_1
      (Input|EnableInput (Game|GetPlayerController 0)))))

(event Input|KeyboardEvents|E
  (params (Key :type Key%20Structure :default "None")))

(fn ConstructionScript)